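; Player character Blueprint that handles walking, camera look and stamina-limited sprinting.
; BeginPlay registers the Enhanced Input context IMC_Player and caches the default walk speed; move and look actions drive yaw-relative movement and controller rotation.
; Holding sprint raises MaxWalkSpeed and drains stamina, restoring default speed at zero.
; Tick regenerates stamina when not sprinting, with 0.1-second Delay nodes throttling both regen and drain.
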(event `self.ReceiveTick`
  (params (DeltaSeconds :type "Float (single-precision)"))
  ; Constant Regen Stamina.
  (if (not (`self.IsSprinting`))
    (`self.RegenStamina`)))

(event `self.ReceiveBeginPlay`
  (bind _returnvalue (pcsubsystem `EnhancedInputLocalPlayerSubsystem` (`GameplayStatics.GetPlayerController` 0)))
  ; Search Main Input Mapping Context of the Player.
  (`/Engine/EditorBlueprintResources/StandardMacros.IsValid` _returnvalue
    (:`Is Valid`
      (message `EnhancedInputSubsystemInterface.AddMappingContext` _returnvalue "/Game/Blueprints/Player/Input/IMC_Player.IMC_Player" 0 (struct))
      ; Set default speed of the player.
      (set `self.DefaultMovementSpeed` (`CharacterMovementComponent.MaxWalkSpeed` (`self.CharacterMovement`))))))

(event `EnhancedInput|/Game/Blueprints/Player/Input/IA_Move`
  (params (ActionValue :type "Vector2D Structure") (ElapsedSeconds :type "Float (double-precision)") (TriggeredSeconds :type "Float (double-precision)") (InputAction :type "InputAction Object Reference" :default "/Game/Blueprints/Player/Input/IA_Move.IA_Move"))
  ; Movement System for player controls.
  (:`Triggered`
    (`self.AddMovementInput` (`KismetMathLibrary.GetRightVector` (`KismetMathLibrary.MakeRotator` (.roll (`self.GetControlRotation`)) 0.0 (.yaw (`self.GetControlRotation`)))) ActionValue_X)
    (`self.AddMovementInput` (`KismetMathLibrary.GetForwardVector` (`KismetMathLibrary.MakeRotator` 0.0 0.0 (.yaw (`self.GetControlRotation`)))) ActionValue_Y)))

(event `EnhancedInput|/Game/Blueprints/Player/Input/IA_Look`
  (params (ActionValue :type "Vector2D Structure") (ElapsedSeconds :type "Float (double-precision)") (TriggeredSeconds :type "Float (double-precision)") (InputAction :type "InputAction Object Reference" :default "/Game/Blueprints/Player/Input/IA_Look.IA_Look"))
  ; Rotation Camera System for player controls.
  (:`Triggered`
    (`self.AddControllerYawInput` ActionValue_X)
    (`self.AddControllerPitchInput` ActionValue_Y)))

(event `EnhancedInput|/Game/Blueprints/Player/Input/IA_Sprint`
  (params (ActionValue :type Boolean) (ElapsedSeconds :type "Float (double-precision)") (TriggeredSeconds :type "Float (double-precision)") (InputAction :type "InputAction Object Reference" :default "/Game/Blueprints/Player/Input/IA_Sprint.IA_Sprint"))
  ; Sprint System for player controls.
  (:`Triggered`
    (if (> (`self.Stamina`) 0.0)
      (set `self.IsSprinting` true)
      (set `CharacterMovementComponent.MaxWalkSpeed` (`self.SprintMovementSpeed`) (`self.CharacterMovement`))
      (`self.DrainStamina`)))
  (:`Completed`
    (set `self.IsSprinting` false)
    (set `CharacterMovementComponent.MaxWalkSpeed` (`self.DefaultMovementSpeed`) (`self.CharacterMovement`))))

(event `DrainStamina`
  ; Drain System of the stamina of the player
  (`KismetSystemLibrary.Delay` 0.1)
  (bind _output_get (set `self.Stamina` (`KismetMathLibrary.FClamp` (- (`self.Stamina`) 3.0) 0.0 (`self.MaxStamina`))))
  (if (== _output_get 0.0)
    (set `CharacterMovementComponent.MaxWalkSpeed` (`self.DefaultMovementSpeed`) (`self.CharacterMovement`))))

(event `RegenStamina`
  ; Regen System of the stamina of the player
  (`KismetSystemLibrary.Delay` 0.1)
  (set `self.Stamina` (`KismetMathLibrary.FClamp` (+ (`self.Stamina`) 2.0) 0.0 (`self.MaxStamina`)))
  (set `CharacterMovementComponent.MaxWalkSpeed` (`self.DefaultMovementSpeed`) (`self.CharacterMovement`)))

(fn `UserConstructionScript`)